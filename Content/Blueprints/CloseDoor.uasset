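; CloseDoor is a one-shot trigger volume that shuts sliding doors behind the player.
; When a PlayerCharacter overlaps its box, it clears the linked lever's on and broken flags and hides the lever mesh.
; It then toggles the first sliding door to false, does the same for an optional second door, and destroys itself.
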(event `self.Box.OnComponentBeginOverlap`
  (params (OverlappedComponent :type "PrimitiveComponent Object Reference") (OtherActor :type "Actor Object Reference") (OtherComp :type "PrimitiveComponent Object Reference") (OtherBodyIndex :type Integer) (bFromSweep :type Boolean) (SweepResult :type "HitResult Structure (by ref)"))
  (bind _lever (`self.lever`))
  (bind _slidingdoor2 (`self.slidingDoor2`))
  (cast `/Game/Blueprints/PlayerAndGame/PlayerCharacter` OtherActor)
  (set `/Game/Blueprints/Lever.IsLeverOn` false _lever)
  (set `/Game/Blueprints/Lever.IsLeverBroken` false _lever)
  (`SceneComponent.SetVisibility` (`/Game/Blueprints/Lever.Mesh - Lever` _lever) false false)
  (`/Game/Blueprints/SlidingDoor.Toggle` (`self.slidingDoor1`) false)
  (`/Engine/EditorBlueprintResources/StandardMacros.IsValid` _slidingdoor2
    (:`Is Valid`
      (`/Game/Blueprints/SlidingDoor.Toggle` _slidingdoor2 false))
    (:`Is Not Valid`
      _))
  (`self.K2_DestroyActor`))

(fn `UserConstructionScript`)