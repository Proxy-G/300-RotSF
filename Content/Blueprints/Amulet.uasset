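; Amulet is a pickup that the player collects by overlapping its sphere or by interacting with it.
; Both paths run the same logic: flag the EndTrigger as having the amulet, restore the Rope and show its mesh, print a message about returning to the boat, then destroy the actor.
; Tick slowly spins the static mesh around its yaw axis while it waits to be collected.
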(event `self.Sphere.OnComponentBeginOverlap`
  (params (OverlappedComponent :type "PrimitiveComponent Object Reference") (OtherActor :type "Actor Object Reference") (OtherComp :type "PrimitiveComponent Object Reference") (OtherBodyIndex :type Integer) (bFromSweep :type Boolean) (SweepResult :type "HitResult Structure (by ref)"))
  (bind _rope (`self.rope`))
  (cast `/Game/Blueprints/PlayerAndGame/PlayerCharacter` OtherActor)
  (set `/Game/Blueprints/EndTrigger.amuletGotten` true (`self.endTrigger`) :!label _label)
  (set `/Game/Blueprints/ClimbableRope.isMissingRope` false _rope)
  (`SceneComponent.SetVisibility` (`/Game/Blueprints/ClimbableRope.Mesh - Rope` _rope) true false)
  (`KismetSystemLibrary.PrintString` "Amulet gotten! I just need to get back to the boat..." true true (struct :`G` 0.66 :`B` 1.0 :`A` 1.0) 5.0)
  (`self.K2_DestroyActor`))

(event `/Game/Blueprints/Interface/IPlayerCanLookAtAndInteractWith.PlayerWantsToInteract`
  (params (PlayerCharacter :type "/Game/Blueprints/PlayerAndGame/PlayerCharacter Object Reference"))
  (goto _label))

(event `self.ReceiveTick`
  (params (DeltaSeconds :type "Float (single-precision)"))
  (bind _staticmesh (`self.StaticMesh`))
  (`SceneComponent.K2_SetRelativeTransform` _staticmesh (`KismetMathLibrary.MakeTransform` (0.0 0.0 0.0) (`KismetMathLibrary.MakeRotator` 0.0 0.0 (+ (.yaw (.rotation (`SceneComponent.GetRelativeTransform` _staticmesh))) (* DeltaSeconds 25.0)))) false false))

(fn `UserConstructionScript`)